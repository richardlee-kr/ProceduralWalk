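; BP_ProceduralWall is a generated dynamic mesh actor that builds a building wall with window and door openings using Geometry Script.
; On rebuild, Loadxml reads window and door bounding boxes from example.xml, converting 256-unit image coordinates into wall space.
; Boolean subtraction cuts each opening from a box, and recessed window boxes are appended with their own material ID.
; The mesh is then scaled by Width, Depth and Height and given wall and window materials.
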(event `self.ReceiveBeginPlay`)

(event `self.OnRebuildGeneratedMesh`
  (params (TargetMesh :type "DynamicMesh Object Reference"))
  (bind _returnvalue (`GeometryScriptLibrary_MeshPrimitiveFunctions.AppendBox` TargetMesh (struct) (struct) 100.0 100.0 100.0 0 0 0 "Base" null))
  (bind _arr (`self.loadxml` "window"))
  (for _array_element _arr
    (bind _returnvalue_2 (`self.makebooleanmesh` _array_element 3.0))
    (`GeometryScriptLibrary_MeshBooleanFunctions.ApplyMeshBoolean` _returnvalue (struct) _returnvalue_2 (struct) "Subtract" (struct) null)
    (bind _returnvalue_3 (`self.makewindow` _array_element 1.4 20.0))
    (`GeometryScriptLibrary_MeshBasicEditFunctions.AppendMesh` _returnvalue _returnvalue_3 (struct) false null))
  (bind _arr_2 (`self.loadxml` "door"))
  (for _array_element_2 _arr_2
    (bind _returnvalue_4 (`self.makebooleanmesh` _array_element_2 1.0))
    (bind _returnvalue_5 (`GeometryScriptLibrary_MeshBooleanFunctions.ApplyMeshBoolean` _returnvalue (struct) _returnvalue_4 (struct) "Subtract" (struct) null)))
  (`GeometryScriptLibrary_MeshTransformFunctions.ScaleMesh` _returnvalue_5 (`KismetMathLibrary.MakeVector` (`self.width`) (`self.depth`) (`self.height`)) null)
  (`DynamicMeshComponent.ConfigureMaterialSet` (`self.DynamicMeshComponent`) (`|MakeArray` (`self.wall_texture`) (`self.window_texture`))))

(fn `loadxml`
  (params (class :type String))
  (returns (arr :type "Array of Vector4 Structure"))
  (locals (windows :type "Array of Vector4 Structure"))
  (bind _windows (`local.windows`))
  (bind (_errormessage _returnvalue) (`EasyXMLParseManager.LoadFromFile` "example.xml")
    (:`Successed`
      (bind _returnvalue_2 (`EasyXMLElement.ReadElements` _returnvalue (`KismetStringLibrary.Concat_StrStr` "facade." class))
        (:`Found`
          (for _array_element _returnvalue_2
            (bind _returnvalue_3 (`EasyXMLElement.ReadElement` _array_element "bndbox")
              (:`Found`
                (bind _returnvalue_4 (`KismetMathLibrary.MakeVector4` (`KismetMathLibrary.Conv_IntToDouble` (`EasyXMLElement.ReadInt` _returnvalue_3 "xmin" 0)) (`KismetMathLibrary.Conv_IntToDouble` (`EasyXMLElement.ReadInt` _returnvalue_3 "xmax" 0)) (`KismetMathLibrary.Conv_IntToDouble` (`EasyXMLElement.ReadInt` _returnvalue_3 "ymin" 0)) (`KismetMathLibrary.Conv_IntToDouble` (`EasyXMLElement.ReadInt` _returnvalue_3 "ymax" 0))))
                (`KismetArrayLibrary.Array_AddUnique` _windows _returnvalue_4)
                (bind (_x _y _z _w) (`KismetMathLibrary.BreakVector4` _returnvalue_4))
                (`KismetSystemLibrary.PrintString` (`KismetStringLibrary.Concat_StrStr` (`KismetStringLibrary.Conv_DoubleToString` _x) "/" (`KismetStringLibrary.Conv_DoubleToString` _y) "/" (`KismetStringLibrary.Conv_DoubleToString` _z) "/" (`KismetStringLibrary.Conv_DoubleToString` _w))))))
          (return _windows))))))

(fn `makebooleanmesh`
  (params (InVec :type "Vector4 Structure (by ref)") (depth :type "Float (double-precision)"))
  (returns (ReturnValue :type "DynamicMesh Object Reference"))
  (bind (_x _y _z _w) (`KismetMathLibrary.BreakVector4` InVec))
  (bind _returnvalue (* (/ (- _w _z) 256.0) 100.0))
  (bind _returnvalue_2 (* (/ (- _y _x) 256.0) 100.0))
  (bind _returnvalue_3 (`self.AllocateComputeMesh`))
  (bind _returnvalue_4 (`GeometryScriptLibrary_MeshPrimitiveFunctions.AppendBox` _returnvalue_3 (struct) (`KismetMathLibrary.MakeTransform` (0.0 0.0 0.0)) 100.0 100.0 100.0 0 0 0 "Base" null))
  (bind _returnvalue_5 (`GeometryScriptLibrary_MeshTransformFunctions.TransformMesh` _returnvalue_4 (`KismetMathLibrary.MakeTransform` (`KismetMathLibrary.MakeVector` -50.0 (+ (- (* (/ _x 256.0) 100.0) 50.0) (/ _returnvalue_2 2.0)) (- (- 100.0 (* (/ _z 256.0) 100.0)) _returnvalue)) (struct) (`KismetMathLibrary.MakeVector` (/ depth 100.0) (/ _returnvalue_2 100.0) (/ _returnvalue 100.0))) null))
  (return _returnvalue_5))

(fn `makewindow`
  (params (InVec :type "Vector4 Structure (by ref)") (depth :type "Float (double-precision)") (windowsize :type "Float (double-precision)"))
  (returns (ReturnValue :type "DynamicMesh Object Reference"))
  (bind (_x _y _z _w) (`KismetMathLibrary.BreakVector4` InVec))
  (bind _returnvalue (* (/ (- _w _z) 256.0) 100.0))
  (bind _returnvalue_2 (* (/ (- _y _x) 256.0) 100.0))
  (bind _returnvalue_3 (`self.AllocateComputeMesh`))
  (bind _returnvalue_4 (`GeometryScriptLibrary_MeshPrimitiveFunctions.AppendBox` _returnvalue_3 (struct) (`KismetMathLibrary.MakeTransform` (0.0 0.0 0.0)) 100.0 100.0 100.0 0 0 0 "Base" null))
  (bind _returnvalue_5 (`GeometryScriptLibrary_MeshTransformFunctions.TransformMesh` _returnvalue_4 (`KismetMathLibrary.MakeTransform` (`KismetMathLibrary.MakeVector` (+ (+ depth -50.0) (/ windowsize 2.0)) (+ (- (* (/ _x 256.0) 100.0) 50.0) (/ _returnvalue_2 2.0)) (- (- 100.0 (* (/ _z 256.0) 100.0)) _returnvalue)) (struct) (`KismetMathLibrary.MakeVector` (/ windowsize 100.0) (/ _returnvalue_2 100.0) (/ _returnvalue 100.0))) null))
  (bind _returnvalue_6 (`GeometryScriptLibrary_MeshMaterialFunctions.RemapMaterialIDs` _returnvalue_5 0 1 null))
  (return _returnvalue_6))

(fn `UserConstructionScript`)