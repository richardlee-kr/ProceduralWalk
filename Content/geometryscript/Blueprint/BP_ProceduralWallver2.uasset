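; Geometry Script generated-mesh actor that rebuilds a four-walled building with windows and doors from facade annotations.
; Each wall reads XML bounding boxes from a hard-coded desktop folder, boolean-cuts openings, inserts window and door meshes, then is rotated and appended.
; Per-wall material ID offsets map slots to glass, black doors or PNG textures imported from that folder.
; BakeStaticMesh copies the result into a static mesh asset.
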(event `self.ReceiveBeginPlay`)

(event `self.OnRebuildGeneratedMesh`
  (params (TargetMesh :type "DynamicMesh Object Reference"))
  (bind _dynamicmeshcomponent (`self.DynamicMeshComponent`))
  (bind _returnvalue (`self.make_wall2` TargetMesh (`self.width`) (`self.depth`) (`self.height`)))
  (bind _returnvalue_2 (`self.AllocateComputeMesh`))
  (bind _returnvalue_3 (`self.make_wall2` _returnvalue_2 (`self.width`) (`self.depth`) (`self.height`) 180.0 16))
  (bind _returnvalue_4 (`GeometryScriptLibrary_MeshBasicEditFunctions.AppendMesh` _returnvalue _returnvalue_3 (struct) false null))
  (bind _returnvalue_5 (`self.AllocateComputeMesh`))
  (bind _returnvalue_6 (`self.make_wall2` _returnvalue_5 (`self.depth`) (`self.width`) (`self.height`) 90.0 32))
  (bind _returnvalue_7 (`GeometryScriptLibrary_MeshBasicEditFunctions.AppendMesh` _returnvalue_4 _returnvalue_6 (struct) false null))
  (bind _returnvalue_8 (`self.AllocateComputeMesh`))
  (bind _returnvalue_9 (`self.make_wall2` _returnvalue_8 (`self.depth`) (`self.width`) (`self.height`) -90.0 48))
  (`GeometryScriptLibrary_MeshBasicEditFunctions.AppendMesh` _returnvalue_7 _returnvalue_9 (struct) false null)
  (for _index (range 64)
    (bind _returnvalue_10 (mod _index 16))
    (if (== _returnvalue_10 15)
      (`PrimitiveComponent.CreateDynamicMaterialInstance` _dynamicmeshcomponent _index "/Game/geometryscript/Material/glass_test.glass_test" "None")
      (elif (== _returnvalue_10 1)
        (bind _returnvalue_11 (`PrimitiveComponent.CreateDynamicMaterialInstance` _dynamicmeshcomponent _index "/Game/geometryscript/Material/wall_test.wall_test" "None"))
        (`MaterialInstanceDynamic.SetTextureParameterValue` _returnvalue_11 "wall_texture" "/Game/MSPresets/M_MS_Glass_Material/Textures/Black.Black")
        (else
          (bind _returnvalue_12 (`KismetRenderingLibrary.ImportFileAsTexture2D` (`KismetStringLibrary.Concat_StrStr` "C:\\Users\\chltm\\OneDrive\\바탕 화면\\test\\" (`KismetStringLibrary.Concat_StrStr` (`KismetStringLibrary.Conv_IntToString` _index) ".png"))))
          (bind _returnvalue_13 (`PrimitiveComponent.CreateDynamicMaterialInstance` _dynamicmeshcomponent _index "/Game/geometryscript/Material/wall_test.wall_test" "None"))
          (`MaterialInstanceDynamic.SetTextureParameterValue` _returnvalue_13 "wall_texture" _returnvalue_12))))))

(fn `applydoor`
  (params (InputPin :type "DynamicMesh Object Reference") (materialoffset :type Integer) (scale :type "Float (double-precision)"))
  (bind _returnvalue (/ 5.0 scale))
  (bind _pos_arr (`self.load_facade_xml` "door" materialoffset))
  (for _array_element _pos_arr
    (bind _returnvalue_2 (`self.makebooleanmesh` _array_element (* _returnvalue 3.0)))
    (`GeometryScriptLibrary_MeshBooleanFunctions.ApplyMeshBoolean` InputPin (struct) _returnvalue_2 (struct) "Subtract" (struct) null)
    (bind _returnvalue_3 (`self.makemesh` _array_element (* _returnvalue 1.0) 20.0 (+ materialoffset 1)))
    (`GeometryScriptLibrary_MeshBasicEditFunctions.AppendMesh` InputPin _returnvalue_3 (struct) false null))
  (return))

(fn `applywindow`
  (params (InputPin :type "DynamicMesh Object Reference") (materialoffset :type Integer) (scale :type "Float (double-precision)"))
  (bind _returnvalue (/ 5.0 scale))
  (bind (_pos_arr _id_arr) (`self.load_facade_xml` "window" materialoffset))
  (for (_array_element _array_index) _pos_arr
    (bind _returnvalue_2 (`self.makebooleanmesh` _array_element (* _returnvalue 5.0)))
    (`GeometryScriptLibrary_MeshBooleanFunctions.ApplyMeshBoolean` InputPin (struct) _returnvalue_2 (struct) "Subtract" (struct) null)
    (bind _returnvalue_3 (`self.makemesh` _array_element (* _returnvalue 2.0) 20.0 (+ materialoffset (`|GetArrayItem` _id_arr _array_index) 2)))
    (`GeometryScriptLibrary_MeshBasicEditFunctions.AppendMesh` InputPin _returnvalue_3 (struct) false null))
  (return))

(fn `applywindow_pane`
  (params (InputPin :type "DynamicMesh Object Reference") (materialoffset :type Integer) (scale :type "Float (double-precision)"))
  (bind _pos_arr (`self.load_window_xml` "window_pane" materialoffset))
  (for _array_element _pos_arr
    (bind _returnvalue (`self.makebooleanmesh` _array_element (* (/ 5.0 scale) 5.0)))
    (bind _returnvalue_2 (`GeometryScriptLibrary_MeshBooleanFunctions.ApplyMeshBoolean` InputPin (struct) _returnvalue (struct) "Subtract" (struct) null))
    (bind _returnvalue_3 (`self.AllocateComputeMesh`))
    (bind _returnvalue_4 (`GeometryScriptLibrary_MeshPrimitiveFunctions.AppendBox` _returnvalue_3 (struct) (`KismetMathLibrary.MakeTransform` (0.5 0.0 0.0)) 100.0 100.0 100.0 0 0 0 "Base" null))
    (bind _returnvalue_5 (`GeometryScriptLibrary_MeshMaterialFunctions.RemapMaterialIDs` _returnvalue_4 0 15 null))
    (`GeometryScriptLibrary_MeshBooleanFunctions.ApplyMeshBoolean` _returnvalue_2 (struct) _returnvalue_5 (struct) "Union" (struct) null))
  (return))

(fn `Bake_static_mesh`
  (bind _to_static_mesh_asset (`self.To Static Mesh Asset`))
  (bind _returnvalue (`BaseDynamicMeshComponent.GetDynamicMesh` (`self.DynamicMeshComponent`)))
  (`/Engine/EditorBlueprintResources/StandardMacros.IsValid` _to_static_mesh_asset
    (:`Is Valid`
      (`GeometryScriptLibrary_StaticMeshFunctions.CopyMeshToStaticMesh` _returnvalue _to_static_mesh_asset (struct) (struct) null))))

(fn `load_facade_xml`
  (params (class :type String) (offset :type Integer))
  (returns (Pos_arr :type "Array of Vector4 Structure") (ID_arr :type "Array of Integer"))
  (locals (windows :type "Array of Vector4 Structure") (IDs :type "Array of Integer"))
  (bind _windows (`local.windows`))
  (bind (_errormessage _returnvalue) (`EasyXMLParseManager.LoadFromFile` (`KismetStringLibrary.Concat_StrStr` "C:\\Users\\chltm\\OneDrive\\바탕 화면\\test\\" (`KismetStringLibrary.Conv_IntToString` offset) ".xml") true)
    (:`Successed`
      (bind _returnvalue_2 (`EasyXMLElement.ReadElements` _returnvalue (`KismetStringLibrary.Concat_StrStr` "facade." class))
        (:`Found`
          (for _array_element _returnvalue_2
            (bind _returnvalue_3 (`EasyXMLElement.ReadElement` _array_element "bndbox")
              (:`Found`
                (bind _returnvalue_4 (`KismetMathLibrary.MakeVector4` (`KismetMathLibrary.Conv_IntToDouble` (`EasyXMLElement.ReadInt` _returnvalue_3 "xmin" 0)) (`KismetMathLibrary.Conv_IntToDouble` (`EasyXMLElement.ReadInt` _returnvalue_3 "xmax" 0)) (`KismetMathLibrary.Conv_IntToDouble` (`EasyXMLElement.ReadInt` _returnvalue_3 "ymin" 0)) (`KismetMathLibrary.Conv_IntToDouble` (`EasyXMLElement.ReadInt` _returnvalue_3 "ymax" 0))))
                (`KismetArrayLibrary.Array_AddUnique` _windows _returnvalue_4)
                (`KismetArrayLibrary.Array_Add` (`local.IDs`) (`EasyXMLElement.ReadInt` _array_element "ID" -1))
                (bind (_x _y _z _w) (`KismetMathLibrary.BreakVector4` _returnvalue_4))
                (`KismetSystemLibrary.PrintString` (`KismetStringLibrary.Concat_StrStr` (`KismetStringLibrary.Conv_DoubleToString` _x) "/" (`KismetStringLibrary.Conv_DoubleToString` _y) "/" (`KismetStringLibrary.Conv_DoubleToString` _z) "/" (`KismetStringLibrary.Conv_DoubleToString` _w))))))
          (return _windows (`local.IDs`)))))))

(fn `load_window_xml`
  (params (class :type String) (offset :type Integer))
  (returns (Pos_arr :type "Array of Vector4 Structure"))
  (locals (windows :type "Array of Vector4 Structure") (IDs :type "Array of Integer"))
  (bind _windows (`local.windows`))
  (bind (_errormessage _returnvalue) (`EasyXMLParseManager.LoadFromFile` (`KismetStringLibrary.Concat_StrStr` "C:\\Users\\chltm\\OneDrive\\바탕 화면\\test\\" (`KismetStringLibrary.Conv_IntToString` offset) ".xml") true)
    (:`Successed`
      (bind _returnvalue_2 (`EasyXMLElement.ReadElements` _returnvalue (`KismetStringLibrary.Concat_StrStr` "window." class))
        (:`Found`
          (for _array_element _returnvalue_2
            (bind _returnvalue_3 (`EasyXMLElement.ReadElement` _array_element "bndbox")
              (:`Found`
                (bind _returnvalue_4 (`KismetMathLibrary.MakeVector4` (`KismetMathLibrary.Conv_IntToDouble` (`EasyXMLElement.ReadInt` _returnvalue_3 "xmin" 0)) (`KismetMathLibrary.Conv_IntToDouble` (`EasyXMLElement.ReadInt` _returnvalue_3 "xmax" 0)) (`KismetMathLibrary.Conv_IntToDouble` (`EasyXMLElement.ReadInt` _returnvalue_3 "ymin" 0)) (`KismetMathLibrary.Conv_IntToDouble` (`EasyXMLElement.ReadInt` _returnvalue_3 "ymax" 0))))
                (`KismetArrayLibrary.Array_AddUnique` _windows _returnvalue_4)
                (bind (_x _y _z _w) (`KismetMathLibrary.BreakVector4` _returnvalue_4))
                (`KismetSystemLibrary.PrintString` (`KismetStringLibrary.Concat_StrStr` (`KismetStringLibrary.Conv_DoubleToString` _x) "/" (`KismetStringLibrary.Conv_DoubleToString` _y) "/" (`KismetStringLibrary.Conv_DoubleToString` _z) "/" (`KismetStringLibrary.Conv_DoubleToString` _w))))))
          (return _windows))))))

(fn `make_wall`
  (params (TargetMesh :type "DynamicMesh Object Reference") (width :type "Float (double-precision)") (depth :type "Float (double-precision)") (height :type "Float (double-precision)") (materialoffset :type Integer))
  (returns (ReturnValue :type "DynamicMesh Object Reference"))
  (bind _returnvalue (`GeometryScriptLibrary_MeshPrimitiveFunctions.AppendBox` TargetMesh (struct) (struct) 100.0 100.0 100.0 0 0 0 "Base" null))
  (bind _returnvalue_2 (`GeometryScriptLibrary_MeshMaterialFunctions.RemapMaterialIDs` _returnvalue 0 (+ materialoffset 0) null))
  (`self.applywindow` _returnvalue_2 materialoffset width)
  (`self.applydoor` _returnvalue_2 materialoffset width)
  (bind _returnvalue_3 (`GeometryScriptLibrary_MeshTransformFunctions.ScaleMesh` _returnvalue_2 (`KismetMathLibrary.MakeVector` width depth height) null))
  (bind _returnvalue_4 (`GeometryScriptLibrary_MeshTransformFunctions.TranslateMesh` _returnvalue_3 (-0.01 0.0 0.0) null))
  (return _returnvalue_4))

(fn `make_wall2`
  (params (TargetMesh :type "DynamicMesh Object Reference") (width :type "Float (single-precision)") (depth :type "Float (single-precision)") (height :type "Float (single-precision)") (angle :type "Float (single-precision)") (materialoffset :type Integer))
  (returns (ReturnValue :type "DynamicMesh Object Reference"))
  (bind _returnvalue (`self.make_wall` TargetMesh width depth height materialoffset))
  (bind _returnvalue_2 (`self.AllocateComputeMesh`))
  (bind _returnvalue_3 (`GeometryScriptLibrary_MeshPrimitiveFunctions.AppendBox` _returnvalue_2 (struct) (`KismetMathLibrary.MakeTransform` (`KismetMathLibrary.MakeVector` (* width 2.0))) (* width 98.0) (* depth 100.0) (* height 100.0) 0 0 0 "Base" null))
  (bind _returnvalue_4 (`GeometryScriptLibrary_MeshBooleanFunctions.ApplyMeshBoolean` _returnvalue (struct) _returnvalue_3 (struct) "Subtract" (struct) null))
  (bind _returnvalue_5 (`GeometryScriptLibrary_MeshTransformFunctions.TransformMesh` _returnvalue_4 (`KismetMathLibrary.MakeTransform` (0.0 0.0 0.0) (`KismetMathLibrary.MakeRotator` 0.0 0.0 angle)) null))
  (return _returnvalue_5))

(fn `makebooleanmesh`
  (params (InVec :type "Vector4 Structure (by ref)") (depth :type "Float (double-precision)"))
  (returns (ReturnValue :type "DynamicMesh Object Reference"))
  (bind (_x _y _z _w) (`KismetMathLibrary.BreakVector4` InVec))
  (bind _returnvalue (* (/ (- _w _z) 256.0) 100.0))
  (bind _returnvalue_2 (* (/ (- _y _x) 256.0) 100.0))
  (bind _returnvalue_3 (`self.AllocateComputeMesh`))
  (bind _returnvalue_4 (`GeometryScriptLibrary_MeshPrimitiveFunctions.AppendBox` _returnvalue_3 (struct) (`KismetMathLibrary.MakeTransform` (0.0 0.0 0.0)) 100.0 100.0 100.0 0 0 0 "Base" null))
  (bind _returnvalue_5 (`GeometryScriptLibrary_MeshTransformFunctions.TransformMesh` _returnvalue_4 (`KismetMathLibrary.MakeTransform` (`KismetMathLibrary.MakeVector` -50.0 (+ (- (* (/ _x 256.0) 100.0) 50.0) (/ _returnvalue_2 2.0)) (- (- 100.0 (* (/ _z 256.0) 100.0)) _returnvalue)) (struct) (`KismetMathLibrary.MakeVector` (/ depth 100.0) (/ _returnvalue_2 100.0) (/ _returnvalue 100.0))) null))
  (return _returnvalue_5))

(fn `makemesh`
  (params (InVec :type "Vector4 Structure (by ref)") (depth :type "Float (double-precision)") (windowsize :type "Float (double-precision)") (materilaID :type Integer))
  (returns (ReturnValue :type "DynamicMesh Object Reference"))
  (bind (_x _y _z _w) (`KismetMathLibrary.BreakVector4` InVec))
  (bind _returnvalue (* (/ (- _w _z) 256.0) 100.0))
  (bind _returnvalue_2 (* (/ (- _y _x) 256.0) 100.0))
  (bind _returnvalue_3 (`self.AllocateComputeMesh`))
  (bind _returnvalue_4 (`GeometryScriptLibrary_MeshPrimitiveFunctions.AppendBox` _returnvalue_3 (struct) (`KismetMathLibrary.MakeTransform` (0.0 0.0 0.0)) 100.0 100.0 100.0 0 0 0 "Base" null))
  (`self.applywindow_pane` _returnvalue_4 materilaID depth)
  (bind _returnvalue_5 (`GeometryScriptLibrary_MeshTransformFunctions.ScaleMesh` _returnvalue_4 (`KismetMathLibrary.MakeVector` (/ windowsize 100.0) (/ _returnvalue_2 100.0) (/ _returnvalue 100.0)) null))
  (bind _returnvalue_6 (`GeometryScriptLibrary_MeshTransformFunctions.TransformMesh` _returnvalue_5 (`KismetMathLibrary.MakeTransform` (`KismetMathLibrary.MakeVector` (+ (+ depth -50.0) (/ windowsize 2.0)) (+ (- (* (/ _x 256.0) 100.0) 50.0) (/ _returnvalue_2 2.0)) (- (- 100.0 (* (/ _z 256.0) 100.0)) _returnvalue)) (struct)) null))
  (bind _returnvalue_7 (`GeometryScriptLibrary_MeshMaterialFunctions.RemapMaterialIDs` _returnvalue_6 0 materilaID null))
  (return _returnvalue_7))

(fn `UserConstructionScript`)