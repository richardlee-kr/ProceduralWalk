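; Endless-runner ground tile that randomizes its obstacles and coins across three lanes.
; BeginPlay rolls a layout: one rock, two barricades plus coins, coins only, or empty; SpawnCoins places child actors at flat or jump arrow rows.
; Player overlap with BoxCollider asks the GameMode for another tile, then destroys this one after a delay.
; Barricade and right-rock hits kill the player; two other death handlers are unconnected.
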(event `self.ReceiveBeginPlay`
  (bind _rock_mid (`self.Rock_Mid`))
  (bind _barricade_left (`self.Barricade_left`))
  (bind _barricade_left_2 (`self.Barricade_left`))
  (bind _barricade_mid (`self.Barricade_mid`))
  (bind _barricade_right (`self.Barricade_right`))
  (bind _rock_left (`self.Rock_Left`))
  (bind _rock_right (`self.Rock_Right`))
  (bind _barricade_mid_2 (`self.Barricade_mid`))
  (bind _barricade_right_2 (`self.Barricade_right`))
  (switch `int` (`KismetMathLibrary.RandomIntegerInRange` 0 8)
    (:`0`
      (`SceneComponent.SetVisibility` _rock_left true false)
      (`PrimitiveComponent.SetCollisionEnabled` _rock_left "QueryAndPhysics")
      (`PrimitiveComponent.SetCollisionProfileName` _rock_left "BlockAll" true)
      (`ActorComponent.SetComponentTickEnabled` _rock_left true))
    (:`1`
      (`SceneComponent.SetVisibility` _rock_mid true false)
      (`PrimitiveComponent.SetCollisionEnabled` _rock_mid "QueryAndPhysics")
      (`PrimitiveComponent.SetCollisionProfileName` _rock_mid "BlockAll" true)
      (`ActorComponent.SetComponentTickEnabled` _rock_mid true))
    (:`2`
      (`SceneComponent.SetVisibility` _rock_right true false)
      (`PrimitiveComponent.SetCollisionEnabled` _rock_right "QueryAndPhysics")
      (`ActorComponent.SetComponentTickEnabled` _rock_right true))
    (:`3`
      (`SceneComponent.SetVisibility` _barricade_left true false)
      (`PrimitiveComponent.SetCollisionEnabled` _barricade_left "QueryAndPhysics")
      (`ActorComponent.SetComponentTickEnabled` _barricade_left true)
      (`SceneComponent.SetVisibility` _barricade_mid true false)
      (`PrimitiveComponent.SetCollisionEnabled` _barricade_mid "QueryAndPhysics")
      (`ActorComponent.SetComponentTickEnabled` _barricade_mid true)
      (`self.SpawnCoins` (`KismetArrayLibrary.Array_Random` (`self.LeftMidCoins`))))
    (:`4`
      (`SceneComponent.SetVisibility` _barricade_mid_2 true false)
      (`PrimitiveComponent.SetCollisionEnabled` _barricade_mid_2 "QueryAndPhysics")
      (`ActorComponent.SetComponentTickEnabled` _barricade_mid_2 true)
      (`SceneComponent.SetVisibility` _barricade_right true false)
      (`PrimitiveComponent.SetCollisionEnabled` _barricade_right "QueryAndPhysics")
      (`ActorComponent.SetComponentTickEnabled` _barricade_right true)
      (`self.SpawnCoins` (`KismetArrayLibrary.Array_Random` (`self.MidRightCoins`))))
    (:`5`
      (`SceneComponent.SetVisibility` _barricade_right_2 true false)
      (`PrimitiveComponent.SetCollisionEnabled` _barricade_right_2 "QueryAndPhysics")
      (`ActorComponent.SetComponentTickEnabled` _barricade_right_2 true)
      (`SceneComponent.SetVisibility` _barricade_left_2 true false)
      (`PrimitiveComponent.SetCollisionEnabled` _barricade_left_2 "QueryAndPhysics")
      (`ActorComponent.SetComponentTickEnabled` _barricade_left_2 true)
      (`self.SpawnCoins` (`KismetArrayLibrary.Array_Random` (`self.LeftRightCoins`))))
    (:`6`
      (`self.SpawnCoins` (`KismetArrayLibrary.Array_Random` (`self.DefaultCoins`))))))

(event `self.BoxCollider.OnComponentBeginOverlap`
  (params (OverlappedComponent :type "PrimitiveComponent Object Reference") (OtherActor :type "Actor Object Reference") (OtherComp :type "PrimitiveComponent Object Reference") (OtherBodyIndex :type Integer) (bFromSweep :type Boolean) (SweepResult :type "HitResult Structure (by ref)"))
  (cast `/Game/ThirdPersonBP/Blueprints/ThirdPersonCharacter` OtherActor)
  (bind _asthird_person_game_mode (cast `/Game/ThirdPersonBP/Blueprints/ThirdPersonGameMode` (`GameplayStatics.GetGameMode`)))
  (`/Game/ThirdPersonBP/Blueprints/ThirdPersonGameMode.AddGroundTile` _asthird_person_game_mode)
  (`KismetSystemLibrary.Delay` 3.0)
  (`self.K2_DestroyActor`))

(event `self.Barricade_right.OnComponentHit`
  (params (HitComponent :type "PrimitiveComponent Object Reference") (OtherActor :type "Actor Object Reference") (OtherComp :type "PrimitiveComponent Object Reference") (NormalImpulse :type "Vector Structure") (Hit :type "HitResult Structure (by ref)"))
  (bind _asthird_person_character (cast `/Game/ThirdPersonBP/Blueprints/ThirdPersonCharacter` OtherActor))
  (`/Game/ThirdPersonBP/Blueprints/ThirdPersonCharacter.PlayerDeath` _asthird_person_character))

(event `self.Barricade_left.OnComponentHit`
  (params (HitComponent :type "PrimitiveComponent Object Reference") (OtherActor :type "Actor Object Reference") (OtherComp :type "PrimitiveComponent Object Reference") (NormalImpulse :type "Vector Structure") (Hit :type "HitResult Structure (by ref)"))
  (bind _asthird_person_character (cast `/Game/ThirdPersonBP/Blueprints/ThirdPersonCharacter` OtherActor))
  (`/Game/ThirdPersonBP/Blueprints/ThirdPersonCharacter.PlayerDeath` _asthird_person_character))

(event `self.Barricade_mid.OnComponentHit`
  (params (HitComponent :type "PrimitiveComponent Object Reference") (OtherActor :type "Actor Object Reference") (OtherComp :type "PrimitiveComponent Object Reference") (NormalImpulse :type "Vector Structure") (Hit :type "HitResult Structure (by ref)"))
  (bind _asthird_person_character (cast `/Game/ThirdPersonBP/Blueprints/ThirdPersonCharacter` OtherActor))
  (`/Game/ThirdPersonBP/Blueprints/ThirdPersonCharacter.PlayerDeath` _asthird_person_character))

(event `self.Rock_Right.OnComponentHit`
  (params (HitComponent :type "PrimitiveComponent Object Reference") (OtherActor :type "Actor Object Reference") (OtherComp :type "PrimitiveComponent Object Reference") (NormalImpulse :type "Vector Structure") (Hit :type "HitResult Structure (by ref)"))
  (bind _asthird_person_character (cast `/Game/ThirdPersonBP/Blueprints/ThirdPersonCharacter` OtherActor))
  (`/Game/ThirdPersonBP/Blueprints/ThirdPersonCharacter.PlayerDeath` _asthird_person_character))

(fn `GetArrowTransform`
  (returns (ArrowTransform :type "Transform Structure"))
  (return (`SceneComponent.K2_GetComponentToWorld` (`self.Arrow`))))

(fn `SpawnCoins`
  (params (Type :type Integer))
  (bind _array (`|MakeArray` (`SceneComponent.GetRelativeTransform` (`self.Arrow17`)) (`SceneComponent.GetRelativeTransform` (`self.Arrow21`)) (`SceneComponent.GetRelativeTransform` (`self.Arrow20`)) (`SceneComponent.GetRelativeTransform` (`self.Arrow19`)) (`SceneComponent.GetRelativeTransform` (`self.Arrow18`))))
  (bind _array_2 (`|MakeArray` (`SceneComponent.GetRelativeTransform` (`self.Arrow6`)) (`SceneComponent.GetRelativeTransform` (`self.Arrow10`)) (`SceneComponent.GetRelativeTransform` (`self.Arrow7`)) (`SceneComponent.GetRelativeTransform` (`self.Arrow9`)) (`SceneComponent.GetRelativeTransform` (`self.Arrow8`))))
  (bind _array_3 (`|MakeArray` (`SceneComponent.GetRelativeTransform` (`self.Arrow5`)) (`SceneComponent.GetRelativeTransform` (`self.Arrow4`)) (`SceneComponent.GetRelativeTransform` (`self.Arrow3`)) (`SceneComponent.GetRelativeTransform` (`self.Arrow2`)) (`SceneComponent.GetRelativeTransform` (`self.Arrow1`))))
  (bind _array_4 (`|MakeArray` (`SceneComponent.GetRelativeTransform` (`self.Arrow11`)) (`SceneComponent.GetRelativeTransform` (`self.Arrow15`)) (`SceneComponent.GetRelativeTransform` (`self.Arrow14`)) (`SceneComponent.GetRelativeTransform` (`self.Arrow13`)) (`SceneComponent.GetRelativeTransform` (`self.Arrow12`))))
  (bind _array_5 (`|MakeArray` (`SceneComponent.GetRelativeTransform` (`self.Arrow30`)) (`SceneComponent.GetRelativeTransform` (`self.Arrow29`)) (`SceneComponent.GetRelativeTransform` (`self.Arrow28`)) (`SceneComponent.GetRelativeTransform` (`self.Arrow27`)) (`SceneComponent.GetRelativeTransform` (`self.Arrow26`))))
  (bind _array_6 (`|MakeArray` (`SceneComponent.GetRelativeTransform` (`self.Arrow16`)) (`SceneComponent.GetRelativeTransform` (`self.Arrow25`)) (`SceneComponent.GetRelativeTransform` (`self.Arrow24`)) (`SceneComponent.GetRelativeTransform` (`self.Arrow23`)) (`SceneComponent.GetRelativeTransform` (`self.Arrow22`))))
  (switch `int` Type
    (:`Default`
      (`KismetSystemLibrary.PrintString` "Hello")
      (return))
    (:`0`
      ;[1 1 1] Flat_Left
      (for (_ _array_index) _array_2
        (`AddComponent|NODE_AddChildActorComponent-0` :`RelativeTransform` (`|GetArrayItem` _array_2 _array_index))))
    (:`1`
      ;[1 1 1] Flat_Mid
      (for (_ _array_index_2) _array_3
        (`AddComponent|NODE_AddChildActorComponent-1` :`RelativeTransform` (`|GetArrayItem` _array_3 _array_index_2))))
    (:`2`
      ;[1 1 1] Flat_Right
      (for (_ _array_index_3) _array_4
        (`AddComponent|NODE_AddChildActorComponent-2` :`RelativeTransform` (`|GetArrayItem` _array_4 _array_index_3))))
    (:`3`
      ;[1 1 1] Jump_Left
      (for (_ _array_index_4) _array_5
        (`AddComponent|NODE_AddChildActorComponent-3` :`RelativeTransform` (`|GetArrayItem` _array_5 _array_index_4))))
    (:`4`
      ;[1 1 1] Jump_Mid
      (for (_ _array_index_5) _array_6
        (`AddComponent|NODE_AddChildActorComponent-4` :`RelativeTransform` (`|GetArrayItem` _array_6 _array_index_5))))
    (:`5`
      ;[1 1 1] Jump_Right
      (for (_ _array_index_6) _array
        (`AddComponent|NODE_AddChildActorComponent-5` :`RelativeTransform` (`|GetArrayItem` _array _array_index_6))))))

(fn `UserConstructionScript`)