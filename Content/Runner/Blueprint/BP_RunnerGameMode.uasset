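; Runner game mode that builds the endless-runner track from chained tiles, spawning an initial stretch at BeginPlay, and keeps a coin count.
; AddGroundTile spawns each piece at the stored arrow transform, then casts it to its tile type to read the next attach point.
; A counter inserts a random left or right corner after eight ground tiles.
; Ground selection always uses the first TileArray entry, as its random range is pinned to zero.
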(event `self.ReceiveBeginPlay`
  (for _ (range 6)
    (`self.AddGroundTile`)))

(fn `AddCoins`
  (set `self.CurretnCoins` (+ (`self.CurretnCoins`) 1)))

(fn `AddGroundTile`
  (bind _cornertilearray (`self.CornerTileArray`))
  (if (> (`self.CurrentTile`) 7)
    (bind _returnvalue (`|SpawnActorFromClass` (`|GetArrayItem` _cornertilearray (`KismetMathLibrary.RandomIntegerInRange` 0 (`KismetArrayLibrary.Array_LastIndex` _cornertilearray))) (`self.NewArrowTransform`) "Undefined" "OverrideRootScale" null null))
    (bind _asbp_left_corner (cast `/Game/Runner/Blueprint/BP_LeftCorner` _returnvalue)
      (:`then`
        (bind _arrowtransform (`/Game/Runner/Blueprint/BP_LeftCorner.GetArrowTransform` _asbp_left_corner))
        (set `self.NewArrowTransform` _arrowtransform))
      (:`CastFailed`
        (bind _asbp_right_corner (cast `/Game/Runner/Blueprint/BP_RightCorner` _returnvalue))
        (bind _arrowtransform_2 (`/Game/Runner/Blueprint/BP_RightCorner.GetArrowTransform` _asbp_right_corner))
        (set `self.NewArrowTransform` _arrowtransform_2)))
    (set `self.CurrentTile` 0)
    (else
      (bind _returnvalue_2 (`|SpawnActorFromClass` (`|GetArrayItem` (`self.TileArray`) (`KismetMathLibrary.RandomIntegerInRange` 0)) (`self.NewArrowTransform`) "Undefined" "OverrideRootScale" null null))
      (bind _asbp_ground_tile (cast `/Game/Runner/Blueprint/BP_GroundTile` _returnvalue_2)
        (:`then`
          (bind _arrowtransform_3 (`/Game/Runner/Blueprint/BP_GroundTile.GetArrowTransform` _asbp_ground_tile))
          (set `self.NewArrowTransform` _arrowtransform_3))
        (:`CastFailed`
          (bind _asbp_ground_up_tile (cast `/Game/Runner/Blueprint/BP_GroundUpTile` _returnvalue_2)
            (:`then`
              (bind _arrowtransform_4 (`/Game/Runner/Blueprint/BP_GroundUpTile.GetArrowTransform` _asbp_ground_up_tile))
              (set `self.NewArrowTransform` _arrowtransform_4))
            (:`CastFailed`
              (bind _asbp_ground_down_tile (cast `/Game/Runner/Blueprint/BP_GroundDownTile` _returnvalue_2))
              (bind _arrowtransform_5 (`/Game/Runner/Blueprint/BP_GroundDownTile.GetArrowTransform` _asbp_ground_down_tile))
              (set `self.NewArrowTransform` _arrowtransform_5)))))
      (set `self.CurrentTile` (+ (`self.CurrentTile`) 1)))))

(fn `UserConstructionScript`)